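; GameMode_PZ is a game mode Blueprint that creates the on-screen UI and holds level progression values.
; On BeginPlay it creates a BP_UI widget and adds it to the viewport.
; Every Tick, while GrowCount is a multiple of ten, it derives Level from GrowCount and resets HP in proportion to that Level.
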(event EventBeginPlay
  (bind _returnvalue (UserInterface|CreateWidget "/Game/BluePrint/BP_UI.BP_UI_C"))
  (UserInterface|Viewport|AddtoViewport _returnvalue 0))

(event EventTick
  (params (DeltaSeconds :type Float%20%28single-precision%29))
  (if (== 0 (Math|Integer|%(Integer) (Variables|Default|GetGrowCount) 10))
    (Variables|Default|SetLevel (+ 1 (/ (Variables|Default|GetGrowCount) 10)))
    (Variables|Default|SetHP (+ 0 (* (Variables|Default|GetLevel) 200)))))

(fn ConstructionScript)