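; Player controller for a PZ game mode that turns spacebar presses into a grow counter.
; On BeginPlay it caches the game mode cast to GameMode_PZ.
; A spacebar press increments the game mode's GrowCount and prints a debug message, but only while both its Starting and StartGrowing flags are set.
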(event EventBeginPlay
  (bind _asgame_mode_pz (Utilities|Casting|CastToGameMode_PZ (Game|GetGameMode)))
  (Variables|Default|SetAs%20Game%20Mode%20PZ _asgame_mode_pz))

(event EventTick
  (params (DeltaSeconds :type Float%20%28single-precision%29)))

(event Input|ActionEvents|InputActionMy_SpaceBar
  (params (Key :type Key%20Structure :default "None"))
  (:Pressed
    (if (Variables|/Game/BluePrint/GameMode_PZ.GameMode_PZ_C|GetStarting (Variables|Default|GetAs%20Game%20Mode%20PZ))
      (if (Variables|/Game/BluePrint/GameMode_PZ.GameMode_PZ_C|GetStartGrowing (Variables|Default|GetAs%20Game%20Mode%20PZ))
        (Variables|/Game/BluePrint/GameMode_PZ.GameMode_PZ_C|SetGrowCount (Variables|Default|GetAs%20Game%20Mode%20PZ) (+ 1 (Variables|/Game/BluePrint/GameMode_PZ.GameMode_PZ_C|GetGrowCount (Variables|Default|GetAs%20Game%20Mode%20PZ))))
        (Development|PrintString "Grow!!")))))

(event Input|ActionEvents|InputActionMy_Right
  (params (Key :type Key%20Structure :default "None")))

(fn ConstructionScript)